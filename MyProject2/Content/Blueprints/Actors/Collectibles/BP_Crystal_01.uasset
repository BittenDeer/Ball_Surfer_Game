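; Collectible crystal that gets pulled into the player when the player pawn overlaps its sphere, then destroys itself.
; The overlap plays a timeline whose curves drive the actor's location toward the player, its scale toward zero and its point light toward dark.
; Each update lerps from current values rather than cached starting ones, so the motion compounds and follows a moving player.
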(event `self.Sphere.OnComponentBeginOverlap`
  (params (OverlappedComponent :type "PrimitiveComponent Object Reference") (OtherActor :type "Actor Object Reference") (OtherComp :type "PrimitiveComponent Object Reference") (OtherBodyIndex :type Integer) (bFromSweep :type Boolean) (SweepResult :type "HitResult Structure (by ref)"))
  (if (== OtherActor (`GameplayStatics.GetPlayerPawn` 0))
    (bind (_direction _crystal_location _crystal_scale _pointlightchange) (`Timeline|Crystal_transform`)
      (:`Update`
        (`self.Crystal_location_change` _crystal_location)
        (`self.CrystalScaleChange` _crystal_scale)
        (`self.Crystal Change Light` _pointlightchange))
      (:`Finished`
        (`self.K2_DestroyActor`)))))

(fn `Crystal Change Light`
  (params (Alpha :type "Float (double-precision)"))
  (bind _pointlight (`self.PointLight`))
  (`LightComponent.SetIntensity` _pointlight (`KismetMathLibrary.Lerp` (`LightComponentBase.Intensity` _pointlight) 0.0 Alpha)))

(fn `Crystal_location_change`
  (params (Alpha :type "Float (double-precision)"))
  (`self.K2_SetActorLocation` (`KismetMathLibrary.VLerp` (`self.K2_GetActorLocation`) (`self.K2_GetActorLocation` (`GameplayStatics.GetPlayerPawn` 0)) Alpha)))

(fn `CrystalScaleChange`
  (params (Alpha :type "Float (double-precision)"))
  (`self.SetActorScale3D` (`KismetMathLibrary.VLerp` (`self.GetActorScale3D`) (0.0 0.0 0.0) Alpha)))

(fn `UserConstructionScript`)