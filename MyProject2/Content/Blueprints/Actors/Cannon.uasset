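; Cannon actor that fires automatically on a repeating FireRate delay from BeginPlay.
; Each shot spawns a BP_Projectile at the Arrow component's location and rotation, scaled by ProjectileScale, with its sphere ignoring the cannon when moving.
; A timeline then animates the barrel's relative location, and both its Update and Finished outputs loop back into the Delay to schedule the next shot.
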(event `self.ReceiveBeginPlay`
  (`KismetSystemLibrary.Delay` (`self.Fire_Rate`) :!label _label)
  (`self.Spawn Projectile`)
  (bind (_direction _cannon_barrel_location) (`Timeline|Cannon Fire Timeline` :!via `PlayFromStart`)
    (:`Update`
      (`self.Cannon Barrel Movement` _cannon_barrel_location)
      (goto _label))
    (:`Finished`
      (goto _label))))

(fn `Cannon Barrel Movement`
  (params (NewLocation_Y :type "Float (double-precision)"))
  (`SceneComponent.K2_SetRelativeLocation` (`self.Cannon_Barrel`) (`KismetMathLibrary.MakeVector` 0.0 NewLocation_Y) false false))

(fn `Spawn Projectile`
  (bind _returnvalue (`|SpawnActorFromClass` "/Game/Blueprints/Actors/Projectiles/BP_Projectile.BP_Projectile_C" (`KismetMathLibrary.MakeTransform` (`SceneComponent.K2_GetComponentLocation` (`self.Arrow`)) (`SceneComponent.K2_GetComponentRotation` (`self.Arrow`)) (`KismetMathLibrary.Conv_DoubleToVector` (`self.Projectile_Scale`))) "AlwaysSpawn" "OverrideRootScale" null null))
  (`PrimitiveComponent.IgnoreActorWhenMoving` (`/Game/Blueprints/Actors/Projectiles/BP_Projectile.Sphere1` _returnvalue) self true))

(fn `UserConstructionScript`)