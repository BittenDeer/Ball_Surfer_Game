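; BP_WinVolume is a trigger volume that completes the level when the player pawn overlaps it with no crystals left.
; It counts remaining BP_Crystal_01 actors and only prints a Polish warning if any are still in the world.
; On completion it finds the current level in the ordered LevelNames array and opens the next entry by name, or quits the game on the last one.
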(event `self.ReceiveActorBeginOverlap`
  (params (OtherActor :type "Actor Object Reference"))
  (if (== OtherActor (`GameplayStatics.GetPlayerPawn` 0))
    (bind _newparam (`self.Check Any Crystals`))
    (if _newparam
      (`KismetSystemLibrary.PrintString` "Nie zebrales krzystalow")
      (else
        (`self.Complete Level`)))))

(fn `Check Any Crystals`
  (returns (NewParam :type Boolean))
  (bind _outactors (`GameplayStatics.GetAllActorsOfClass` "/Game/Blueprints/Actors/Collectibles/BP_Crystal_01.BP_Crystal_01_C"))
  (bind _output_get (set `self.Any_Crystals` (!= (`KismetArrayLibrary.Array_Length` _outactors) 0)))
  (return _output_get))

(fn `Complete Level`
  (if (`self.IsLastLevel`)
    (`KismetSystemLibrary.QuitGame` null "Quit")
    (else
      (`KismetSystemLibrary.PrintString` "NOWY POZIOM")
      (`GameplayStatics.OpenLevel` (`self.Load Next Level`)))))

(fn `CurrentLevelIndex`
  (returns (`Return Value` :type Integer))
  (bind _returnvalue (`GameplayStatics.GetCurrentLevelName` true))
  (return (`KismetArrayLibrary.Array_Find` (`self.LevelNames`) (`KismetStringLibrary.Conv_StringToName` _returnvalue))))

(fn `IsLastLevel`
  (returns (`Return Value` :type Boolean))
  (return (== (`self.CurrentLevelIndex`) (`KismetArrayLibrary.Array_LastIndex` (`self.LevelNames`)))))

(fn `Load Next Level`
  (returns (Output :type Name))
  (return (`|GetArrayItem` (`self.LevelNames`) (+ (`self.CurrentLevelIndex`) 1))))

(fn `UserConstructionScript`)